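; BP_Trunk is a procedural tree trunk actor that scatters BP_LowerBranch actors around itself and attaches them to its Cylinder.
; Each branch gets a random height and X/Y offsets from independent angles scaled by TrunkRadius.
; Pitch and roll follow that offset via look-at, while yaw is random.
; The same NoOfBranches loop runs both in InitialiseTree, called at construction, and again on BeginPlay.
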(event `self.ReceiveBeginPlay`
  (bind _returnvalue (`KismetMathLibrary.RandomFloatInRange` 0.0 360.0))
  (bind _trunkradius (`self.TrunkRadius`))
  (bind (_finalrotation_roll _finalrotation_pitch) (`KismetMathLibrary.BreakRotator` (`self.FinalRotation`)))
  (bind _returnvalue_2 (`SceneComponent.K2_GetComponentLocation` (`self.centrepoint`)))
  (for _ (range (`self.NoOfBranches`))
    (set `self.RandomRotation` _returnvalue)
    (set `self.RandomLocationX` (* (`KismetMathLibrary.DegCos` _returnvalue) _trunkradius))
    (set `self.RandomLocationY` (* _trunkradius (`KismetMathLibrary.DegSin` _returnvalue)))
    (set `self.RandomLocationZ` (`KismetMathLibrary.RandomFloatInRange` 0.0 60.0))
    (set `self.RandomLocationVector` (`KismetMathLibrary.MakeVector` (`self.RandomLocationX`) (`self.RandomLocationY`) (`self.RandomLocationZ`)))
    (set `self.FinalRotation` (`KismetMathLibrary.FindLookAtRotation` _returnvalue_2 (+ _returnvalue_2 (`self.RandomLocationVector`))))
    (bind _returnvalue_3 (`|SpawnActorFromClass` "/Game/BP_LowerBranch.BP_LowerBranch_C" (`KismetMathLibrary.MakeTransform` (`self.RandomLocationVector`) (`KismetMathLibrary.MakeRotator` _finalrotation_roll _finalrotation_pitch (`self.RandomRotation`))) "Undefined" "MultiplyWithRoot" null 0 null))
    (`self.K2_AttachToComponent` _returnvalue_3 (`self.Cylinder`) "None" "KeepRelative" "KeepRelative" "KeepWorld" true)))

(fn `InitialiseTree`
  (bind _returnvalue (`KismetMathLibrary.RandomFloatInRange` 0.0 360.0))
  (bind _trunkradius (`self.TrunkRadius`))
  (bind (_finalrotation_roll _finalrotation_pitch) (`KismetMathLibrary.BreakRotator` (`self.FinalRotation`)))
  (bind _returnvalue_2 (`SceneComponent.K2_GetComponentLocation` (`self.centrepoint`)))
  (for _ (range (`self.NoOfBranches`))
    (set `self.RandomRotation` _returnvalue)
    (set `self.RandomLocationX` (* (`KismetMathLibrary.DegCos` _returnvalue) _trunkradius))
    (set `self.RandomLocationY` (* _trunkradius (`KismetMathLibrary.DegSin` _returnvalue)))
    (set `self.RandomLocationZ` (`KismetMathLibrary.RandomFloatInRange` 0.0 60.0))
    (set `self.RandomLocationVector` (`KismetMathLibrary.MakeVector` (`self.RandomLocationX`) (`self.RandomLocationY`) (`self.RandomLocationZ`)))
    (set `self.FinalRotation` (`KismetMathLibrary.FindLookAtRotation` _returnvalue_2 (+ _returnvalue_2 (`self.RandomLocationVector`))))
    (bind _returnvalue_3 (`|SpawnActorFromClass` "/Game/BP_LowerBranch.BP_LowerBranch_C" (`KismetMathLibrary.MakeTransform` (`self.RandomLocationVector`) (`KismetMathLibrary.MakeRotator` _finalrotation_roll _finalrotation_pitch (`self.RandomRotation`))) "Undefined" "MultiplyWithRoot" null 0 null))
    (`self.K2_AttachToComponent` _returnvalue_3 (`self.Cylinder`) "None" "KeepRelative" "KeepRelative" "KeepWorld" true)))

(fn `UserConstructionScript`
  (`KismetSystemLibrary.PrintString` "2")
  (`self.InitialiseTree`))