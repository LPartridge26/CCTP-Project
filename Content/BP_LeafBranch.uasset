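; BP_LeafBranch is a procedural foliage actor that builds a randomized cluster of green leaf blobs around a pivot.
; Its construction script destroys previously generated components, then picks a leaf count between configurable minimum and maximum values.
; Each leaf is a sphere static mesh with random offset and scale, attached to PivotRoot and tracked in GeneratedLeaves for the next rebuild.
; The event graph holds no active logic.
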(fn `UserConstructionScript`
  (bind _returnvalue (`KismetMathLibrary.RandomFloatInRange` 3.0 3.5))
  (bind _generatedleaves (`self.GeneratedLeaves`))
  (for _array_element _generatedleaves
    (`ActorComponent.K2_DestroyComponent` _array_element))
  (`KismetArrayLibrary.Array_Clear` _generatedleaves)
  (bind _output_get (set `self.LeafCount` (`KismetMathLibrary.RandomIntegerInRange` (`self.LeafCountMin`) (`self.LeafCountMax`))))
  (for _ (range _output_get)
    (bind _returnvalue_2 (`AddComponent|NODE_AddStaticMeshComponent-1` :`RelativeTransform` (`KismetMathLibrary.MakeTransform` (`KismetMathLibrary.MakeVector` (`KismetMathLibrary.RandomFloatInRange` -75.0 75.0) (`KismetMathLibrary.RandomFloatInRange` -75.0 75.0) (`KismetMathLibrary.RandomFloatInRange` 25.0 135.0)) (struct) (`KismetMathLibrary.MakeVector` _returnvalue _returnvalue _returnvalue))))
    (`StaticMeshComponent.SetStaticMesh` _returnvalue_2 "/Game/StarterContent/Props/MaterialSphere.MaterialSphere")
    (`PrimitiveComponent.SetMaterial` _returnvalue_2 0 "/Game/green.green")
    (`SceneComponent.K2_AttachToComponent` _returnvalue_2 (`self.PivotRoot`) "None" "KeepRelative" "KeepRelative" "KeepRelative" true)
    (`KismetArrayLibrary.Array_Add` (`self.GeneratedLeaves`) _returnvalue_2)))