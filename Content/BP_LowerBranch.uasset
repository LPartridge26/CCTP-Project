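; BP_LowerBranch is a procedural tree branch actor that recursively grows child branches from its SpawnPoint.
; SpawnBranches runs from both the Construction Script and BeginPlay, randomly continuing with one child, splitting into two oppositely rolled children, or stopping.
; Each attached child gets random roll and yaw, a depth-based shrinking scale and, for lower branches, an incremented Depth.
; At MaxDepth it spawns a BP_LeafBranch instead.
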(event `self.ReceiveBeginPlay`
  (`self.SpawnBranches`))

(event `SpawnBranches`
  (bind _returnvalue (`KismetMathLibrary.RandomFloatInRange` 0.0 1.0))
  (bind _returnvalue_2 (`SceneComponent.GetRelativeTransform` (`self.SpawnPoint`)))
  (bind _returnvalue_3 (`SceneComponent.GetRelativeTransform` (`self.SpawnPoint`)))
  (bind _returnvalue_4 (`SceneComponent.GetRelativeTransform` (`self.SpawnPoint`)))
  (bind _returnvalue_5 (`KismetMathLibrary.MultiplyMultiply_FloatFloat` 0.95 (`KismetMathLibrary.Conv_IntToDouble` (`self.Depth`))))
  (bind _returnvalue_6 (`KismetMathLibrary.MultiplyMultiply_FloatFloat` 0.95 (`KismetMathLibrary.Conv_IntToDouble` (`self.Depth`))))
  (bind _returnvalue_7 (`KismetMathLibrary.MultiplyMultiply_FloatFloat` 0.95 (`KismetMathLibrary.Conv_IntToDouble` (`self.Depth`))))
  (if (>= (`self.Depth`) (`self.MaxDepth`))
    (bind _returnvalue_8 (`|SpawnActorFromClass` "/Game/BP_LeafBranch.BP_LeafBranch_C" (`KismetMathLibrary.MakeTransform` (.location _returnvalue_3) (`KismetMathLibrary.MakeRotator` (+ (.roll (.rotation _returnvalue_3)) (`KismetMathLibrary.RandomFloatInRange` 10.0 25.0)) (.pitch (.rotation _returnvalue_3)) (`KismetMathLibrary.RandomFloatInRange` 0.0 360.0)) (* (.scale _returnvalue_3) (`KismetMathLibrary.MakeVector` _returnvalue_6 _returnvalue_6 _returnvalue_6))) "Undefined" "MultiplyWithRoot" null null null))
    (`self.K2_AttachToComponent` _returnvalue_8 (`self.SpawnPoint`) "None" "SnapToTarget" "KeepRelative" "KeepRelative" true)
    (elif (<= _returnvalue (`self.ContinueChance`))
      (bind _returnvalue_9 (`|SpawnActorFromClass` "BP_LowerBranch_C" (`KismetMathLibrary.MakeTransform` (.location _returnvalue_4) (`KismetMathLibrary.MakeRotator` (+ (.roll (.rotation _returnvalue_4)) (`KismetMathLibrary.RandomFloatInRange` 15.0 30.0)) (.pitch (.rotation _returnvalue_4)) (`KismetMathLibrary.RandomFloatInRange` 0.0 360.0)) (* (.scale _returnvalue_4) (`KismetMathLibrary.MakeVector` _returnvalue_7 _returnvalue_7 _returnvalue_7))) "Undefined" "MultiplyWithRoot" null (+ (`self.Depth`) 1) null :!label _label))
      (`self.K2_AttachToComponent` _returnvalue_9 (`self.SpawnPoint`) "None" "SnapToTarget" "KeepRelative" "KeepRelative" true)
      (elif (<= _returnvalue (`self.SplitChance`))
        (bind _returnvalue_10 (`|SpawnActorFromClass` "BP_LowerBranch_C" (`KismetMathLibrary.MakeTransform` (.location _returnvalue_2) (`KismetMathLibrary.MakeRotator` (+ (.roll (.rotation _returnvalue_2)) (`KismetMathLibrary.RandomFloatInRange` -15.0 -30.0)) (.pitch (.rotation _returnvalue_2)) (`KismetMathLibrary.RandomFloatInRange` 0.0 360.0)) (* (.scale _returnvalue_2) (`KismetMathLibrary.MakeVector` _returnvalue_5 _returnvalue_5 _returnvalue_5))) "Undefined" "MultiplyWithRoot" null (+ (`self.Depth`) 1) null))
        (`self.K2_AttachToComponent` _returnvalue_10 (`self.SpawnPoint`) "None" "SnapToTarget" "KeepRelative" "KeepRelative" true)
        (goto _label)))))

(fn `UserConstructionScript`
  (`self.SpawnBranches`))